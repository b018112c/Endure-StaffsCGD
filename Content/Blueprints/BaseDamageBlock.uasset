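; BaseDamageBlock is an obstacle Blueprint that damages a VehicleBlueprint according to the speed it loses on impact.
; A Box overlap records approach speed minus a zero-damage threshold, then a Cube hit subtracts current speed and scales the difference into Health damage.
; At zero Health or below, the vehicle despawns with an explosion sound, then respawns after a short delay with Health reset.
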(event `self.Cube.OnComponentHit`
  (params (HitComponent :type "PrimitiveComponent Object Reference") (OtherActor :type "Actor Object Reference") (OtherComp :type "PrimitiveComponent Object Reference") (NormalImpulse :type "Vector Structure") (Hit :type "HitResult Structure (by ref)"))
  ;[1 1 1] Object Damage Dealt
  (bind _asvehicle_blueprint (cast `/Game/Vehicle/VehicleBlueprint` OtherActor))
  (bind _speed (`self.GetSpeed` _asvehicle_blueprint))
  (bind _returnvalue (- (`self.PriorSpeed`) _speed))
  (if (not (< _returnvalue 0))
    (bind _output_get (set `/Game/Vehicle/VehicleBlueprint.Health` (- (`/Game/Vehicle/VehicleBlueprint.Health` _asvehicle_blueprint) (* _returnvalue (/ (`self.DamageMultiplier`) 100.0))) _asvehicle_blueprint))
    (set `self.PriorSpeed` 0)
    (`/Engine/EditorBlueprintResources/StandardMacros.CompareFloat` _output_get
      (:`==`
        _)
      (:`<`
        _))
    (`/Game/Vehicle/VehicleBlueprint.Despawn` _asvehicle_blueprint)
    (`GameplayStatics.PlaySoundAtLocation` "/Game/VehicleAdv/Sound/Explosion_Cue.Explosion_Cue" (`SceneComponent.K2_GetComponentLocation` (`WheeledVehicle.Mesh` _asvehicle_blueprint)))
    (`KismetSystemLibrary.Delay` 0.8)
    (`/Game/Vehicle/VehicleBlueprint.Respawn` _asvehicle_blueprint)
    (set `/Game/Vehicle/VehicleBlueprint.Health` 1.0 _asvehicle_blueprint)))

(event `self.Box.OnComponentBeginOverlap`
  (params (OverlappedComponent :type "PrimitiveComponent Object Reference") (OtherActor :type "Actor Object Reference") (OtherComp :type "PrimitiveComponent Object Reference") (OtherBodyIndex :type Integer) (bFromSweep :type Boolean) (SweepResult :type "HitResult Structure (by ref)"))
  ;[1 1 1] Calculate Speed to be used for damage
  (bind _asvehicle_blueprint (cast `/Game/Vehicle/VehicleBlueprint` OtherActor))
  (bind _speed (`self.GetSpeed` _asvehicle_blueprint))
  (set `self.PriorSpeed` (- _speed (`self.ZeroDamageSpeed`))))

(fn `GetSpeed`
  (params (Car :type "Actor Object Reference"))
  (returns (Speed :type Integer))
  (bind _asvehicle_blueprint (cast `/Game/Vehicle/VehicleBlueprint` Car)
    (:`then`
      (return (`KismetMathLibrary.FFloor` (`KismetMathLibrary.Abs` (* (`WheeledVehicleMovementComponent.GetForwardSpeed` (`WheeledVehicle.VehicleMovement` _asvehicle_blueprint)) 0.022)))))
    (:`CastFailed`
      (return 0))))

(fn `UserConstructionScript`)