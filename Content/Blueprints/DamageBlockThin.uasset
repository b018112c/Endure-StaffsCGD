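; DamageBlockThin is a block actor that moves along a timeline-driven path from its placed position.
; On BeginPlay it stores its starting location and plays the timeline from the start.
; Each update rotates the timeline's vector by the Cube component's world rotation, so motion follows the block's orientation, then sets that offset from the start as relative location without sweeping.
; No damage logic appears in this graph.
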(event `self.ReceiveBeginPlay`
  (set `self.StartLocation` (`self.K2_GetActorLocation`))
  (bind (_direction _newtrack_0) (`Timeline|Timeline_0` :!via `PlayFromStart`)
    (:`Update`
      (`self.K2_SetActorRelativeLocation` (+ (`self.StartLocation`) (`KismetMathLibrary.GreaterGreater_VectorRotator` _newtrack_0 (`SceneComponent.K2_GetComponentRotation` (`self.Cube`))))))))

(fn `UserConstructionScript`
  (`parent.UserConstructionScript`))