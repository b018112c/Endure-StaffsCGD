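; DamageBlock is an obstacle that damages a VehicleBlueprint according to how fast it approaches.
; An overlap Box samples the vehicle's absolute forward speed, converts and floors it, and stores any excess over ZeroDamageSpeed as PriorSpeed.
; On hit, the Cube subtracts PriorSpeed scaled by DamageMultiplier from vehicle Health, resets PriorSpeed and prints "Dead" at zero or below.
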(event `self.Cube.OnComponentHit`
  (params (HitComponent :type "PrimitiveComponent Object Reference") (OtherActor :type "Actor Object Reference") (OtherComp :type "PrimitiveComponent Object Reference") (NormalImpulse :type "Vector Structure") (Hit :type "HitResult Structure (by ref)"))
  ;[1 1 1] Object Damage Dealt
  (bind _asvehicle_blueprint (cast `/Game/VehicleAdvBP/Blueprints/VehicleBlueprint` OtherActor))
  (bind _output_get (set `/Game/VehicleAdvBP/Blueprints/VehicleBlueprint.Health` (- (`/Game/VehicleAdvBP/Blueprints/VehicleBlueprint.Health` _asvehicle_blueprint) (* (`self.PriorSpeed`) (/ (`self.DamageMultiplier`) 100.0))) _asvehicle_blueprint))
  (set `self.PriorSpeed` 0)
  (`/Engine/EditorBlueprintResources/StandardMacros.CompareFloat` _output_get
    (:`==`
      _)
    (:`<`
      _))
  (`KismetSystemLibrary.PrintString` "Dead"))

(event `self.Box.OnComponentBeginOverlap`
  (params (OverlappedComponent :type "PrimitiveComponent Object Reference") (OtherActor :type "Actor Object Reference") (OtherComp :type "PrimitiveComponent Object Reference") (OtherBodyIndex :type Integer) (bFromSweep :type Boolean) (SweepResult :type "HitResult Structure (by ref)"))
  ;[1 1 1] Calculate Speed to be used for damage
  (bind _asvehicle_blueprint (cast `/Game/VehicleAdvBP/Blueprints/VehicleBlueprint` OtherActor))
  (bind _returnvalue (- (`KismetMathLibrary.FFloor` (`KismetMathLibrary.Abs` (* (`WheeledVehicleMovementComponent.GetForwardSpeed` (`WheeledVehicle.VehicleMovement` _asvehicle_blueprint)) 0.022))) (`self.ZeroDamageSpeed`)))
  (if (not (< _returnvalue 0))
    (set `self.PriorSpeed` _returnvalue)))

(fn `UserConstructionScript`)