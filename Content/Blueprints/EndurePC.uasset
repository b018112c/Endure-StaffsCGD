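; Player controller for a vehicle game that routes input to the player's VehicleBlueprint and manages menus.
; Cast helpers fetch the pawn or its movement component for driving, strafing, boosting and element cycling.
; Camera axes rotate the spring arm or reset it to its pitch, and another input toggles in-car view.
; It also starts the game, opens main, settings and pause widgets, and debug-prints GameStarted every tick.
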(event EventBeginPlay)

(event EventTick
  (params (DeltaSeconds :type Float%20%28single-precision%29))
  (Development|PrintString (Utilities|String|ToString(Boolean) (Variables|Default|GetGameStarted))))

(event Input|ActionEvents|InputActionHandbrake
  (params (Key :type Key%20Structure :default "AnyKey"))
  ;[1 1 1] Steering
  (:Pressed
    (bind _vehiclemovement (CallFunction|GetMovement))
    (Class|WheeledVehicleMovementComponent|SetHandbrakeInput _vehiclemovement true))
  (:Released
    (bind _vehiclemovement_2 (CallFunction|GetMovement))
    (Class|WheeledVehicleMovementComponent|SetHandbrakeInput _vehiclemovement_2 false)))

(event Input|ActionEvents|InputActionBoostHold
  (params (Key :type Key%20Structure :default "AnyKey"))
  ;[1 1 1] Boost
  (:Pressed
    (bind _asvehicle_blueprint (CallFunction|GetBlueprint))
    (Default|BoostColourPress _asvehicle_blueprint))
  (:Released
    (bind _asvehicle_blueprint_2 (CallFunction|GetBlueprint))
    (Default|BoostColourRelease _asvehicle_blueprint_2)))

(event Input|ActionEvents|InputActionStrafe_Left
  (params (Key :type Key%20Structure :default "AnyKey"))
  ;[1 1 1] Strafe
  (:Pressed
    (bind _asvehicle_blueprint (CallFunction|GetBlueprint))
    (Default|StrafeLeft _asvehicle_blueprint)))

(event Input|ActionEvents|InputActionStrafe_Right
  (params (Key :type Key%20Structure :default "AnyKey"))
  ;[1 1 1] Strafe
  (:Pressed
    (bind _asvehicle_blueprint (CallFunction|GetBlueprint))
    (Default|StrafeRight _asvehicle_blueprint)))

(event Input|ActionEvents|InputActionSwitchCamera
  (params (Key :type Key%20Structure :default "AnyKey"))
  ;[1 1 1] Handles Camera Movement
  (:Pressed
    (bind _asvehicle_blueprint (CallFunction|GetBlueprint))
    (Default|EnableIncarView _asvehicle_blueprint (not (Variables|/Game/Vehicle/VehicleBlueprint.VehicleBlueprint_C|GetIsInCar _asvehicle_blueprint)))))

(event Input|ActionEvents|InputActionPauseKey
  (params (Key :type Key%20Structure :default "AnyKey"))
  (:Pressed
    (CallFunction|PauseGame)))

(event Input|ActionEvents|InputActionElementCycleRight
  (params (Key :type Key%20Structure :default "AnyKey"))
  ;[1 1 1] ElementChanging
  (:Pressed
    (bind _asvehicle_blueprint (CallFunction|GetBlueprint))
    (Default|ElementCycle _asvehicle_blueprint 1)))

(event Input|ActionEvents|InputActionElementCycleLeft
  (params (Key :type Key%20Structure :default "AnyKey"))
  ;[1 1 1] ElementChanging
  (:Pressed
    (bind _asvehicle_blueprint (CallFunction|GetBlueprint))
    (Default|ElementCycle _asvehicle_blueprint -1)))

(event Input|AxisEvents|InputAxisCameraYawFB
  (params (AxisValue :type Float%20%28single-precision%29))
  ;[1 1 1] Handles Camera Movement
  (bind _asvehicle_blueprint (CallFunction|GetBlueprint))
  (if (Math|Vector|NotEqual(Vector) (Math|Vector|MakeVector AxisValue (stale Input|AxisEvents|InputAxisCameraYawLR AxisValue) 0.0) "0, 0, 0" 0.0001)
    (Transformation|SetRelativeRotation (Variables|/Game/Vehicle/VehicleBlueprint.VehicleBlueprint_C|GetSpringArm _asvehicle_blueprint) (Math|Rotator|MakeRotationfromAxes (Math|Vector|MakeVector AxisValue (stale Input|AxisEvents|InputAxisCameraYawLR AxisValue) 0.0) "0, 0, 0" "0, 0, 0") false false)
    (Transformation|AddLocalRotation (Variables|/Game/Vehicle/VehicleBlueprint.VehicleBlueprint_C|GetSpringArm _asvehicle_blueprint) (Variables|/Game/Vehicle/VehicleBlueprint.VehicleBlueprint_C|GetCameraPitch _asvehicle_blueprint) false false)
    (else
      (Transformation|SetRelativeRotation (Variables|/Game/Vehicle/VehicleBlueprint.VehicleBlueprint_C|GetSpringArm _asvehicle_blueprint) (Variables|/Game/Vehicle/VehicleBlueprint.VehicleBlueprint_C|GetCameraPitch _asvehicle_blueprint) false false))))

(event Input|AxisEvents|InputAxisCameraYawLR
  (params (AxisValue :type Float%20%28single-precision%29))
  ;[1 1 1] Handles Camera Movement
  (bind _asvehicle_blueprint (CallFunction|GetBlueprint))
  (if (Math|Vector|NotEqual(Vector) (Math|Vector|MakeVector (stale Input|AxisEvents|InputAxisCameraYawFB AxisValue) AxisValue 0.0) "0, 0, 0" 0.0001)
    (Transformation|SetRelativeRotation (Variables|/Game/Vehicle/VehicleBlueprint.VehicleBlueprint_C|GetSpringArm _asvehicle_blueprint) (Math|Rotator|MakeRotationfromAxes (Math|Vector|MakeVector (stale Input|AxisEvents|InputAxisCameraYawFB AxisValue) AxisValue 0.0) "0, 0, 0" "0, 0, 0") false false)
    (Transformation|AddLocalRotation (Variables|/Game/Vehicle/VehicleBlueprint.VehicleBlueprint_C|GetSpringArm _asvehicle_blueprint) (Variables|/Game/Vehicle/VehicleBlueprint.VehicleBlueprint_C|GetCameraPitch _asvehicle_blueprint) false false)
    (else
      (Transformation|SetRelativeRotation (Variables|/Game/Vehicle/VehicleBlueprint.VehicleBlueprint_C|GetSpringArm _asvehicle_blueprint) (Variables|/Game/Vehicle/VehicleBlueprint.VehicleBlueprint_C|GetCameraPitch _asvehicle_blueprint) false false))))

(event Input|AxisEvents|InputAxisMoveForward
  (params (AxisValue :type Float%20%28single-precision%29))
  ;[1 1 1] Steering
  (bind _vehiclemovement (CallFunction|GetMovement))
  (Class|WheeledVehicleMovementComponent|SetThrottleInput _vehiclemovement AxisValue))

(event Input|AxisEvents|InputAxisMoveRight
  (params (AxisValue :type Float%20%28single-precision%29))
  ;[1 1 1] Steering
  (bind _vehiclemovement (CallFunction|GetMovement))
  (Class|WheeledVehicleMovementComponent|SetSteeringInput _vehiclemovement AxisValue))

(event Input|AxisEvents|InputAxisBoost
  (params (AxisValue :type Float%20%28single-precision%29))
  ;[1 1 1] Boost
  (bind _asvehicle_blueprint (CallFunction|GetBlueprint))
  (Default|BoostPress _asvehicle_blueprint AxisValue))

(fn ConstructionScript)

(fn GetMovement
  (bind _aswheeled_vehicle (Utilities|Casting|CastToWheeledVehicle (Game|Player|GetPlayerPawn 0))
    (:then
      (return (Variables|/Script/Engine.WheeledVehicle|GetVehicleMovement _aswheeled_vehicle)))
    (:CastFailed
      (return 0))))

(fn GetBlueprint
  (bind _asvehicle_blueprint (Utilities|Casting|CastToVehicleBlueprint (Game|Player|GetPlayerPawn 0))
    (:then
      (return _asvehicle_blueprint))
    (:CastFailed
      (return 0))))

(fn StartGame
  (Input|SetInputModeGameOnly)
  (Variables|Default|SetGameStarted true)
  (bind _asvehicle_blueprint (Utilities|Casting|CastToVehicleBlueprint (Game|Player|GetPlayerPawn 0))
    (:then
      (Default|StartGame _asvehicle_blueprint)
      (return))
    (:CastFailed
      (return))))

(fn SettingsMenu
  (bind _returnvalue (UserInterface|CreateWidget "/Game/Blueprints/UI/SettingsUI.SettingsUI_C"))
  (UserInterface|Viewport|AddtoViewport _returnvalue 0)
  (Variables|/Script/Engine.PlayerController|SetbShowMouseCursor (Game|GetPlayerController 0) true)
  (return))

(fn MainMenuScreen
  (bind _returnvalue (UserInterface|CreateWidget "/Game/Blueprints/UI/MainMenuUI.MainMenuUI_C"))
  (UserInterface|Viewport|AddtoViewport _returnvalue 0)
  (Variables|/Script/Engine.PlayerController|SetbShowMouseCursor (Game|GetPlayerController 0) true)
  (return))

(fn PauseGame
  (Utilities|IsValid (LocalVariables|GetPauseMenuReference)
    (:Is%20Valid
      _)
    (:Is%20Not%20Valid
      (bind _returnvalue (UserInterface|CreateWidget "/Game/Blueprints/UI/PauseMenuUI.PauseMenuUI_C"))
      (LocalVariables|SetPauseMenuReference _returnvalue)))
  (Input|SetInputModeUIOnly (Game|GetPlayerController 0) (LocalVariables|GetPauseMenuReference) false)
  (UserInterface|Viewport|AddtoViewport (LocalVariables|GetPauseMenuReference) 0)
  (Game|SetGamePaused true)
  (Variables|/Script/Engine.PlayerController|SetbShowMouseCursor (Game|GetPlayerController 0) true)
  (return))